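; Dungeon "AP" room Blueprint that runs a monster encounter and tracks when the room is cleared.
; When a player overlaps CheckPlayer in an uncleared room, it sends room-entered messages to the player's controller and game mode.
; SpawnMosnters spawns the RoomData enemy class at four cached scene points, giving each monster a back-reference to the room.
; MonsterDead counts down the fixed monster total, then sets ClearCondition and notifies both of room completion.
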(event `self.ReceiveBeginPlay`
  ; 초기 몬스터 개수 및 스폰 위치 캐싱
  (`parent.ReceiveBeginPlay`)
  (set `self.MonsterAmount` 4)
  (`KismetArrayLibrary.Array_Add` (`self.MonsterSpawnLocationList`) (`self.Scene`))
  (`KismetArrayLibrary.Array_Add` (`self.MonsterSpawnLocationList`) (`self.Scene1`))
  (`KismetArrayLibrary.Array_Add` (`self.MonsterSpawnLocationList`) (`self.Scene2`))
  (`KismetArrayLibrary.Array_Add` (`self.MonsterSpawnLocationList`) (`self.Scene3`)))

(event `SpawnMosnters`
  (bind (_roomdata_offerskillcount _roomdata_roomlevel _roomdata_enemygroup) (break `/Game/Data/Structure/RoomData/ST_RoomData` (`self.RoomData`)))
  ; 데이터 테이블에서 뽑은 몬스터 BP를 spawn 위치에서 생성
  (for _array_element (`self.MonsterSpawnLocationList`)
    (bind _returnvalue (`|SpawnActorFromClass` _roomdata_enemygroup (`SceneComponent.K2_GetComponentToWorld` _array_element) "AlwaysSpawn" "MultiplyWithRoot" null null))
    (bind _asbp_monster_base (cast `/Game/Blueprints/Pawn/Monster/BP_MonsterBase` _returnvalue))
    (`/Engine/EditorBlueprintResources/StandardMacros.IsValid` _asbp_monster_base
      (:`Is Valid`
        (set `/Game/Blueprints/Pawn/Monster/BP_MonsterBase.RoomData` self _asbp_monster_base)
        (`KismetArrayLibrary.Array_Add` (`self.APMonsterList`) _returnvalue)))))

(event `/Game/Interface/BPI_MonsterDead.MonsterDead`
  ; 죽었을 때 이벤트
  (bind _output_get (set `self.MonsterAmount` (- (`self.MonsterAmount`) 1)))
  (if (and (== _output_get 0) (not (`self.ClearCondition`)))
    (set `self.ClearCondition` true)
    (message `/Game/Interface/BPI_RoomEvent.OnRoomEndCondition` (`self.As GM In Game Mode`) (`self.ClearCondition`) (`self.RoomType`))
    (message `/Game/Interface/BPI_RoomEvent.OnRoomEndCondition` (`GameplayStatics.GetPlayerController` 0) (`self.ClearCondition`) (`self.RoomType`))))

(event `self.CheckPlayer.OnComponentBeginOverlap`
  (params (OverlappedComponent :type "PrimitiveComponent Object Reference") (OtherActor :type "Actor Object Reference") (OtherComp :type "PrimitiveComponent Object Reference") (OtherBodyIndex :type Integer) (bFromSweep :type Boolean) (SweepResult :type "HitResult Structure (by ref)"))
  ; 방 입장했을 경우
  (bind _asbp_player (cast `/Game/Blueprints/Pawn/Player/BP_Player` OtherActor))
  (`/Engine/EditorBlueprintResources/StandardMacros.IsValid` _asbp_player
    (:`Is Valid`
      (if (not (`self.ClearCondition`))
        (message `/Game/Interface/BPI_RoomEvent.OnRoomEntered` (`Pawn.GetController` _asbp_player) (`self.RoomType`) (`self.ClearCondition`) self)
        (message `/Game/Interface/BPI_RoomEvent.OnRoomEntered` (`self.As GM In Game Mode`) (`self.RoomType`) (`self.ClearCondition`) self)))))

(fn `UserConstructionScript`
  (`parent.UserConstructionScript`))
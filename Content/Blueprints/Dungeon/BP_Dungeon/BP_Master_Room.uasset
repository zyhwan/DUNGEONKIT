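; BP_Master_Room is a dungeon room Blueprint that knows its own room type and stores the matching room data.
; On BeginPlay it caches a GM_InGameMode reference, then initializes that data.
; InitRoomData switches on RoomType (AD monster, AP monster, reward, start or boss) and copies a fixed-name row from that type's DataTable into RoomData.
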(event `self.ReceiveBeginPlay`
  (`|ExecutionSequence`
    (:`then_0`
      (`self.InitGameModeRef`))
    (:`then_1`
      (`self.InitRoomData`))))

(fn `InitGameModeRef`
  (bind _asgm_in_game_mode (cast `/Game/Core/GameMode/GM_InGameMode` (`GameplayStatics.GetGameMode`)))
  (`/Engine/EditorBlueprintResources/StandardMacros.IsValid` _asgm_in_game_mode
    (:`Is Valid`
      (set `self.As GM In Game Mode` _asgm_in_game_mode))))

(fn `InitRoomData`
  ; 생성되는 방이 어떤 방인지 데이터 저장. 각 BP가 본인이 무슨방인지 정보를 가지고 있음.
  (switch `/Game/Data/Enum/E_RoomType` (`self.RoomType`)
    (:`NewEnumerator1`
      (bind _returnvalue (`|GetDataTableRow` "/Game/Data/DataTable/RoomData/DT_ADBattleRoomData.DT_ADBattleRoomData" "AD")
        (:`then`
          (set `self.RoomData` _returnvalue))))
    (:`NewEnumerator2`
      (bind _returnvalue_2 (`|GetDataTableRow` "/Game/Data/DataTable/RoomData/DT_APBattleRoomData.DT_APBattleRoomData" "AP")
        (:`then`
          (set `self.RoomData` _returnvalue_2))))
    (:`NewEnumerator3`
      (bind _returnvalue_3 (`|GetDataTableRow` "/Game/Data/DataTable/RoomData/DT_RewardRoomData.DT_RewardRoomData" "Reward")
        (:`then`
          (set `self.RoomData` _returnvalue_3))))
    (:`NewEnumerator10`
      (bind _returnvalue_4 (`|GetDataTableRow` "/Game/Data/DataTable/RoomData/DT_StartRoomData.DT_StartRoomData" "Start")
        (:`then`
          (set `self.RoomData` _returnvalue_4))))
    (:`NewEnumerator11`
      (bind _returnvalue_5 (`|GetDataTableRow` "/Game/Data/DataTable/RoomData/DT_BossRoomData.DT_BossRoomData" "Boss")
        (:`then`
          (set `self.RoomData` _returnvalue_5))))))

(fn `UserConstructionScript`)
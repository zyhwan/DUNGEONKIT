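; Boss room Blueprint for the dungeon, extending a parent room with a single-boss clear condition.
; SpawnBossMonster spawns the RoomData enemy class at the first child of Center and gives the boss a reference back to the room.
; Player overlap with CheckPlayer notifies the game mode while the room is uncleared.
; MonsterDead decrements the count and, at zero, marks the room cleared and notifies the game mode and player controller.
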(event `self.ReceiveBeginPlay`
  ; 몬스터 초기 개수 설정
  (`parent.ReceiveBeginPlay`)
  (set `self.MonsterAmount` 1))

(event `SpawnBossMonster`
  (bind (_roomdata_offerskillcount _roomdata_roomlevel _roomdata_enemygroup) (break `/Game/Data/Structure/RoomData/ST_RoomData` (`self.RoomData`)))
  ; 보스 몬스터 생성
  (bind _returnvalue (`|SpawnActorFromClass` _roomdata_enemygroup (`SceneComponent.K2_GetComponentToWorld` (`SceneComponent.GetChildComponent` (`self.Center`) 0)) "AlwaysSpawn" "MultiplyWithRoot" null null))
  (bind _asbp_boss_monster (cast `/Game/Blueprints/Pawn/Monster/Boss_Monster/BP_BossMonster` _returnvalue))
  (`/Engine/EditorBlueprintResources/StandardMacros.IsValid` _asbp_boss_monster
    (:`Is Valid`
      (set `/Game/Blueprints/Pawn/Monster/BP_MonsterBase.RoomData` self _asbp_boss_monster)
      (set `self.BossMonsterRef` _asbp_boss_monster))))

(event `self.CheckPlayer.OnComponentBeginOverlap`
  (params (OverlappedComponent :type "PrimitiveComponent Object Reference") (OtherActor :type "Actor Object Reference") (OtherComp :type "PrimitiveComponent Object Reference") (OtherBodyIndex :type Integer) (bFromSweep :type Boolean) (SweepResult :type "HitResult Structure (by ref)"))
  ; 방에 입장했을 경우
  (bind _asbp_player (cast `/Game/Blueprints/Pawn/Player/BP_Player` OtherActor))
  (`/Engine/EditorBlueprintResources/StandardMacros.IsValid` _asbp_player
    (:`Is Valid`
      (if (not (`self.ClearCondition`))
        (message `/Game/Interface/BPI_RoomEvent.OnRoomEntered` (`self.As GM In Game Mode`) (`self.RoomType`) (`self.ClearCondition`) self)))))

(event `/Game/Interface/BPI_MonsterDead.MonsterDead`
  ; 몬스터 죽음 이벤트 처리
  (bind _output_get (set `self.MonsterAmount` (- (`self.MonsterAmount`) 1)))
  (if (and (== _output_get 0) (not (`self.ClearCondition`)))
    (set `self.ClearCondition` true)
    (message `/Game/Interface/BPI_RoomEvent.OnRoomEndCondition` (`self.As GM In Game Mode`) (`self.ClearCondition`) (`self.RoomType`))
    (message `/Game/Interface/BPI_RoomEvent.OnRoomEndCondition` (`GameplayStatics.GetPlayerController` 0) (`self.ClearCondition`) (`self.RoomType`))))

(fn `UserConstructionScript`
  (`parent.UserConstructionScript`))
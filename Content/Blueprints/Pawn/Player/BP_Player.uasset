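; Player character with camera-aimed arrow attacks, dash, and a skill-driven buff system.
; Stats and skills load from data tables, and UpdateSkillID applies stat buffs, attack upgrades, orbiting orbs or chain explosion.
; Fire line-traces from the camera to aim arrows, scaling from single to delayed double to three-way spread, while Tick spins evenly spaced orbs.
; Damage subtracts defense and can reflect to attackers, with HP, dash and death pushed to controller UI.
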(event `Set_for_a_Moment_Input`
  ; 방에 입장 했을 때 잠시 멈추기
  (`CharacterMovementComponent.DisableMovement` (`self.CharacterMovement`))
  (set `self.IsAttackTime` false)
  (`KismetSystemLibrary.K2_SetTimerDelegate` (delegate `SetEnableInput`) 3.0))

(event `SetEnableInput`
  ; 방에 입장 했을 때 잠시 멈추기
  (`CharacterMovementComponent.SetMovementMode` (`self.CharacterMovement`) "MOVE_Walking" 0)
  (set `self.IsAttackTime` true))

(event `self.ReceiveBeginPlay`
  ; 플레이어 디폴트 스텟 초기화
  (`self.SetPlayerStat`)
  ; 플레이어 체력 정보 넘기기
  (bind _asbp_player_controller (cast `/Game/Controller/BP_PlayerController` (`GameplayStatics.GetPlayerController` 0)))
  (`/Engine/EditorBlueprintResources/StandardMacros.IsValid` _asbp_player_controller
    (:`Is Valid`
      (set `self.PC_Ref` _asbp_player_controller)
      (`self.SetPlayerHPGUI`)
      ; 플레이어 스킬 데이터 캐싱
      (bind _outrownames (`DataTableFunctionLibrary.GetDataTableRowNames` "/Game/Data/DataTable/SkillData/DT_SkillDetail.DT_SkillDetail"))
      (for _array_element _outrownames
        (bind _returnvalue (`|GetDataTableRow` "/Game/Data/DataTable/SkillData/DT_SkillDetail.DT_SkillDetail" _array_element)
          (:`then`
            (`KismetArrayLibrary.Array_Add` (`self.SkillDatas`) _returnvalue)))))))

(event `EnhancedInput|/Game/Inputs/IA_Fire`
  (params (ActionValue :type Boolean) (ElapsedSeconds :type "Float (double-precision)") (TriggeredSeconds :type "Float (double-precision)") (InputAction :type "InputAction Object Reference" :default "/Game/Inputs/IA_Fire.IA_Fire"))
  ; 발사 로직
  (:`Triggered`
    (if (`self.IsAttackTime`)
      (`self.Fire`))))

(event `Key|Zero`
  (params (Key :type "Key Structure"))
  ; 구체 생성 디버깅
  (:`Pressed`
    (`self.MakeOrb`)))

(event `EnhancedInput|/Game/Inputs/IA_Dash`
  (params (ActionValue :type Boolean) (ElapsedSeconds :type "Float (double-precision)") (TriggeredSeconds :type "Float (double-precision)") (InputAction :type "InputAction Object Reference" :default "/Game/Inputs/IA_Dash.IA_Dash"))
  (bind (_returnvalue_x _returnvalue_y) (`KismetMathLibrary.BreakVector` (* (`self.GetVelocity`) 10.0)))
  ; 플레이어 대시 로직
  (:`Triggered`
    (if (not (`self.IsDashing`))
      (set `self.IsDashing` true)
      (`self.LaunchCharacter` (`KismetMathLibrary.MakeVector` _returnvalue_x _returnvalue_y))
      (`KismetSystemLibrary.K2_SetTimerDelegate` (delegate `SetDashEnable`) 1.0)
      (`self.SetDashEffect`)
      (`/Game/Core/HUD/BP_GameHUD.SetDashAlpha0` (`/Game/Controller/BP_PlayerController.HUD_Ref` (`self.PC_Ref`))))))

(event `self.ReceiveTick`
  (params (DeltaSeconds :type "Float (single-precision)"))
  ; 생성한 구체 이동 로직
  (`self.MoveOrb` DeltaSeconds))

(event `SetDashEnable`
  ; 플레이어 대시 로직
  (set `self.IsDashing` false)
  (`/Game/Core/HUD/BP_GameHUD.SetDashAlpha1` (`/Game/Controller/BP_PlayerController.HUD_Ref` (`self.PC_Ref`))))

(event `self.ReceiveAnyDamage`
  (params (Damage :type "Float (single-precision)") (DamageType :type "DamageType Object Reference") (InstigatedBy :type "Controller Object Reference") (DamageCauser :type "Actor Object Reference"))
  (bind _reflectiveamount (`self.ReflectiveAmount`))
  (bind _returnvalue (- Damage (`self.DEF`)))
  ; 데미지 계산 방어력 보다 받는 데미지가 낮으면 최소 5는 닳게함, 받는 데미지에서 방어력을 뺀 만큼 체력이 깎임
  ;; 체력이 0보다 작아지는지 먼저 체크
  (if (`self.IsDeath`)
    _
    (elif (>= (- (`self.Current_HP`) (- Damage (`self.DEF`))) 0.0)
      ;; 플레이어의 방어력과 몬스터의 공격력 비교 분기문
      (if (<= _returnvalue 0.0)
        (set `self.Current_HP` (- (`self.Current_HP`) 5.0))
        (else
          (set `self.Current_HP` (- (`self.Current_HP`) _returnvalue))))
      (if (> _reflectiveamount 0.0)
        (`GameplayStatics.ApplyDamage` DamageCauser _reflectiveamount null self)
        (`self.SetPlayerHPGUI`)
        (else
          (`self.SetPlayerHPGUI`)))
      (else
        (`self.EventPlayerDie`)))))

(event `Fire`
  ; 기본 공격 강화 로직 포함
  (`self.PlayAnimMontage` "/Game/Blueprints/Pawn/Player/Animations/AM_Player.AM_Player" 1.0 "Fire")
  (switch `int` (`self.AttackLevel`)
    (:`0`
      (`self.Level1_Attack`))
    (:`1`
      (`self.Level1_Attack`)
      (`KismetSystemLibrary.K2_SetTimer` null "Level1_Attack" 0.1))
    (:`2`
      (`self.Level2_Attack`))))

(event `SetPlayerHPGUI`
  ; 플레이어 최대 체력 UI 초기화
  (message `/Game/Interface/BPI_SetPlayerHp.SetPlayerHp` (`self.PC_Ref`) (`self.Current_HP`) (`self.MaxHP`)))

(event `Key|Four`
  (params (Key :type "Key Structure"))
  ; 플레이어 죽음 디버깅
  (:`Pressed`
    (set `self.IsDeath` true :!label _label)
    (set `self.Current_HP` 0.0)
    (`self.SetPlayerHPGUI`)
    (`CharacterMovementComponent.DisableMovement` (`self.CharacterMovement`))
    (`|PlayMontage` (`self.Mesh`) "/Game/Blueprints/Pawn/Player/Animations/AM_Player.AM_Player" 1.0 0.0 "Death"
      (:`then`
        (`/Game/Controller/BP_PlayerController.StartDeathGUI` (`self.PC_Ref`))))))

(event `EventPlayerDie`
  ; 플레이어 죽음 디버깅
  (goto _label))

(event `SetDashEffect`
  (`ActorComponent.Activate` (`self.NS_TrailEffect`) false)
  (`Timeline|DashEffect` :!via `PlayFromStart`
    (:`Finished`
      (`ActorComponent.Deactivate` (`self.NS_TrailEffect`)))))

(fn `FireArrow`
  (locals (TargetLocation :type "Vector Structure"))
  (`self.PlayAnimMontage` "/Game/Blueprints/Pawn/Player/Animations/AM_Player.AM_Player" 1.0 "Fire")
  (switch `int` (`self.AttackLevel`)
    (:`0`
      (`self.Level1_Attack`))
    (:`1`
      (`self.Level1_Attack`)
      (`self.Level1_Attack`))))

(fn `Level1_Attack`
  (locals (Target :type "Vector Structure"))
  (bind _returnvalue (`SceneComponent.GetSocketLocation` (`self.Mesh`) "AttackPoint"))
  (bind _returnvalue_2 (`SceneComponent.GetSocketLocation` (`self.Mesh`) "AttackPoint"))
  (bind _output_get (set `local.Target` (+ (* (`KismetMathLibrary.GetForwardVector` (`SceneComponent.K2_GetComponentRotation` (`self.Camera`))) 3500.0) (`SceneComponent.K2_GetComponentLocation` (`self.Camera`)))))
  (bind _outhit (`KismetSystemLibrary.LineTraceSingle` (`SceneComponent.K2_GetComponentLocation` (`self.Camera`)) _output_get "TraceTypeQuery1"))
  (bind (_bblockinghit _binitialoverlap _time _distance _location) (`GameplayStatics.BreakHitResult` _outhit))
  (if _bblockinghit
    (`|SpawnActorFromClass` "/Game/Blueprints/Actor/BP_Arrow.BP_Arrow_C" (`KismetMathLibrary.MakeTransform` _returnvalue (`KismetMathLibrary.FindLookAtRotation` _returnvalue _location)) "AlwaysSpawn" "MultiplyWithRoot" null self null)
    (else
      (`|SpawnActorFromClass` "/Game/Blueprints/Actor/BP_Arrow.BP_Arrow_C" (`KismetMathLibrary.MakeTransform` _returnvalue_2 (`KismetMathLibrary.FindLookAtRotation` _returnvalue_2 (`local.Target`))) "AlwaysSpawn" "MultiplyWithRoot" null self null))))

(fn `Level2_Attack`
  (locals (TargetPoint :type "Vector Structure"))
  (bind _returnvalue (`SceneComponent.GetSocketLocation` (`self.Mesh`) "AttackPoint"))
  (bind _returnvalue_2 (`SceneComponent.GetSocketLocation` (`self.Mesh`) "AttackPoint"))
  (bind _returnvalue_3 (`SceneComponent.GetSocketLocation` (`self.Mesh`) "AttackPoint"))
  (bind _returnvalue_4 (`SceneComponent.GetSocketLocation` (`self.Mesh`) "AttackPoint"))
  (bind (_returnvalue_roll _returnvalue_pitch _returnvalue_yaw) (`KismetMathLibrary.BreakRotator` (`KismetMathLibrary.FindLookAtRotation` _returnvalue_2 (`local.TargetPoint`))))
  (bind (_returnvalue_roll_2 _returnvalue_pitch_2 _returnvalue_yaw_2) (`KismetMathLibrary.BreakRotator` (`KismetMathLibrary.FindLookAtRotation` _returnvalue_4 (`local.TargetPoint`))))
  (bind _returnvalue_5 (`KismetMathLibrary.MakeRotator` _returnvalue_roll_2 _returnvalue_pitch_2 (+ _returnvalue_yaw_2 -10.0)))
  (bind _returnvalue_6 (`KismetMathLibrary.MakeRotator` _returnvalue_roll _returnvalue_pitch (+ _returnvalue_yaw 10.0)))
  (bind _output_get (set `local.TargetPoint` (+ (* (`KismetMathLibrary.GetForwardVector` (`SceneComponent.K2_GetComponentRotation` (`self.Camera`))) 3500.0) (`SceneComponent.K2_GetComponentLocation` (`self.Camera`)))))
  (bind _outhit (`KismetSystemLibrary.LineTraceSingle` (`SceneComponent.K2_GetComponentLocation` (`self.Camera`)) _output_get "TraceTypeQuery1"))
  (bind (_bblockinghit _binitialoverlap _time _distance _location) (`GameplayStatics.BreakHitResult` _outhit))
  (if _bblockinghit
    (`|SpawnActorFromClass` "/Game/Blueprints/Actor/BP_Arrow.BP_Arrow_C" (`KismetMathLibrary.MakeTransform` _returnvalue (`KismetMathLibrary.FindLookAtRotation` _returnvalue _location)) "AlwaysSpawn" "MultiplyWithRoot" null self null)
    (`|SpawnActorFromClass` "/Game/Blueprints/Actor/BP_Arrow.BP_Arrow_C" (`KismetMathLibrary.MakeTransform` _returnvalue_2 _returnvalue_6) "AlwaysSpawn" "MultiplyWithRoot" null self null)
    (`|SpawnActorFromClass` "/Game/Blueprints/Actor/BP_Arrow.BP_Arrow_C" (`KismetMathLibrary.MakeTransform` _returnvalue_4 _returnvalue_5) "AlwaysSpawn" "MultiplyWithRoot" null self null)
    (else
      (`|SpawnActorFromClass` "/Game/Blueprints/Actor/BP_Arrow.BP_Arrow_C" (`KismetMathLibrary.MakeTransform` _returnvalue_3 (`KismetMathLibrary.FindLookAtRotation` _returnvalue_3 (`local.TargetPoint`))) "AlwaysSpawn" "MultiplyWithRoot" null self null)
      (`|SpawnActorFromClass` "/Game/Blueprints/Actor/BP_Arrow.BP_Arrow_C" (`KismetMathLibrary.MakeTransform` _returnvalue_2 _returnvalue_6) "AlwaysSpawn" "MultiplyWithRoot" null self null)
      (`|SpawnActorFromClass` "/Game/Blueprints/Actor/BP_Arrow.BP_Arrow_C" (`KismetMathLibrary.MakeTransform` _returnvalue_4 _returnvalue_5) "AlwaysSpawn" "MultiplyWithRoot" null self null))))

(fn `MakeOrb`
  (set `self.IsOrb` true)
  (bind _returnvalue (`|SpawnActorFromClass` "/Game/Blueprints/Pawn/Player/BP_Orb.BP_Orb_C" (`self.GetTransform`) "AlwaysSpawn" "MultiplyWithRoot" self null))
  (`KismetArrayLibrary.Array_Add` (`self.OrbRef`) _returnvalue)
  (`self.K2_AttachToComponent` _returnvalue (`self.OrbRoot`) "None" "KeepRelative" "KeepRelative" "KeepRelative" true)
  (`self.UpdateOrbPositions`))

(fn `MakeRotation`
  (bind (_returnvalue_roll _returnvalue_pitch) (`KismetMathLibrary.BreakRotator` (`self.K2_GetActorRotation`)))
  (bind (_returnvalue_roll_2 _returnvalue_pitch_2 _returnvalue_yaw) (`KismetMathLibrary.BreakRotator` (`KismetMathLibrary.RInterpTo_Constant` (`self.K2_GetActorRotation`) (`KismetMathLibrary.FindLookAtRotation` (+ (0.0 0.0 0.0) (0.0 0.0 0.0)) (- (`.ImpactPoint` (`GameplayStatics.BreakHitResult` (`PlayerController.GetHitResultUnderCursorByChannel` (`GameplayStatics.GetPlayerController` 0) "TraceTypeQuery1" true))) (`self.K2_GetActorLocation`))) (`GameplayStatics.GetWorldDeltaSeconds`) (`self.Interp Speed`))))
  (`self.K2_SetActorRotation` (`KismetMathLibrary.MakeRotator` _returnvalue_roll _returnvalue_pitch _returnvalue_yaw)))

(fn `MoveOrb`
  (params (DeltaTime :type "Float (double-precision)"))
  (if (`self.IsOrb`)
    (`SceneComponent.K2_AddRelativeRotation` (`self.OrbRoot`) (`KismetMathLibrary.MakeRotator` 0.0 0.0 (* DeltaTime (`self.OrbSpeed`))) false false)))

(fn `MovePlayer`
  (params (X_Value :type "Float (double-precision)") (Y_Value :type "Float (double-precision)"))
  (bind (_returnvalue_roll _returnvalue_pitch _returnvalue_yaw) (`KismetMathLibrary.BreakRotator` (`self.GetControlRotation`)))
  (bind _returnvalue (`KismetMathLibrary.MakeRotator` 0.0 0.0 _returnvalue_yaw))
  (`self.AddMovementInput` (* X_Value (`KismetMathLibrary.GetForwardVector` _returnvalue)))
  (`self.AddMovementInput` (* Y_Value (`KismetMathLibrary.GetRightVector` _returnvalue))))

(fn `SetAtkBuff`
  (params (BuffData :type "/Game/Data/Structure/SkillData/ST_BuffSkill Structure"))
  (set `self.ATK` (+ (`self.ATK`) BuffData_Increase_Amount_5_77F78A3C4D686F5CEC562791C24B33F7))
  (return))

(fn `SetAttackLevel`
  (if (< (`self.AttackLevel`) 2)
    (set `self.AttackLevel` (+ (`self.AttackLevel`) 1))
    (return)))

(fn `SetChainExplosion`
  (set `self.IsChainExplosion` true))

(fn `SetDefBuff`
  (params (BuffData :type "/Game/Data/Structure/SkillData/ST_BuffSkill Structure"))
  (set `self.DEF` (+ (`self.DEF`) BuffData_Increase_Amount_5_77F78A3C4D686F5CEC562791C24B33F7))
  (return))

(fn `SetHpBuff`
  (params (BuffData :type "/Game/Data/Structure/SkillData/ST_BuffSkill Structure"))
  (bind _returnvalue (+ BuffData_Increase_Amount_5_77F78A3C4D686F5CEC562791C24B33F7 (`self.Current_HP`)))
  ; 만약에 최대 체력보다 커지면 최대 체력을 늘리고 아니라면 현재 체력을 회복
  (if (< _returnvalue (`self.MaxHP`))
    (set `self.Current_HP` _returnvalue)
    (`self.SetPlayerHPGUI`)
    (return)
    (else
      (bind _output_get (set `self.Current_HP` _returnvalue))
      (set `self.MaxHP` _output_get)
      (`self.SetPlayerHPGUI`)
      (return))))

(fn `SetLifeStillAmountBuff`
  (params (BuffData :type "/Game/Data/Structure/SkillData/ST_BuffSkill Structure"))
  (set `self.Life_Steal_Amount` (+ (`self.Life_Steal_Amount`) BuffData_Increase_Amount_5_77F78A3C4D686F5CEC562791C24B33F7))
  (return))

(fn `SetLook`
  (params (`X Value` :type "Float (double-precision)") (`Y Value` :type "Float (double-precision)"))
  (`self.AddControllerYawInput` (`local.X Value`))
  (`self.AddControllerPitchInput` (* (`local.Y Value`) -1.0)))

(fn `SetPlayerStat`
  (bind _returnvalue (`|GetDataTableRow` "/Game/Data/DataTable/PlayerData/DT_PlayerStatData.DT_PlayerStatData" "PlayerDefaultStat")
    (:`then`
      (bind _output_get (set `self.PlayerStat` _returnvalue))
      (`self.SendPlayerStat` (`self.PlayerStat`))
      (`|ExecutionSequence`
        (:`then_0`
          (set `self.Current_HP` (break `/Game/Data/Structure/PlayerData/ST_PlayerStat` _output_get))
          (set `self.MaxHP` (break `/Game/Data/Structure/PlayerData/ST_PlayerStat` _output_get)))
        (:`then_1`
          (set `self.SPEED` (`.Speed_10_BEA2144C40894A17901B9187D844625F` (break `/Game/Data/Structure/PlayerData/ST_PlayerStat` _output_get))))
        (:`then_2`
          (set `self.ATK` (`.ATK_12_C2E6F845422C8DB04EB271A549A7A53B` (break `/Game/Data/Structure/PlayerData/ST_PlayerStat` _output_get))))
        (:`then_3`
          (set `self.DEF` (`.Def_17_AE77776D46D6DCC01E12B39B3DBE6C5F` (break `/Game/Data/Structure/PlayerData/ST_PlayerStat` _output_get))))
        (:`then_4`
          (set `self.Life_Steal_Amount` (`.LifeStealAmount_22_4F0176FC4FE0293A8DB91B8F146C912A` (break `/Game/Data/Structure/PlayerData/ST_PlayerStat` _output_get))))
        (:`then_5`
          (set `self.Dash Cool Time` (`.DashCoolTime_21_76431C9042D2F6D8EA920BB5C9D9C27E` (break `/Game/Data/Structure/PlayerData/ST_PlayerStat` _output_get))))
        (:`then_6`
          (set `self.ReflectiveAmount` (`.ReflectiveAmount_20_54B9E86049B1AAA72A2D9482A019CAAD` (break `/Game/Data/Structure/PlayerData/ST_PlayerStat` _output_get))))))))

(fn `SetReflectiveAmountBuff`
  (params (BuffData :type "/Game/Data/Structure/SkillData/ST_BuffSkill Structure"))
  (set `self.ReflectiveAmount` (+ (`self.ReflectiveAmount`) BuffData_Increase_Amount_5_77F78A3C4D686F5CEC562791C24B33F7))
  (return))

(fn `SetSpeedAndAtkBuff`
  (params (BuffData :type "/Game/Data/Structure/SkillData/ST_BuffSkill Structure"))
  (set `self.ATK` (+ (`self.ATK`) BuffData_Increase_Amount_5_77F78A3C4D686F5CEC562791C24B33F7))
  (set `self.SPEED` (+ (`self.SPEED`) BuffData_Increase_Amount_5_77F78A3C4D686F5CEC562791C24B33F7))
  (return))

(fn `SetSpeedBuff`
  (params (BuffData :type "/Game/Data/Structure/SkillData/ST_BuffSkill Structure"))
  (bind _output_get (set `self.SPEED` (+ (`self.SPEED`) BuffData_Increase_Amount_5_77F78A3C4D686F5CEC562791C24B33F7)))
  (set `CharacterMovementComponent.MaxWalkSpeed` _output_get (`self.CharacterMovement`))
  (return))

(fn `ShowCurrentPlayerStat`
  (`KismetSystemLibrary.PrintString` (`KismetTextLibrary.Conv_TextToString` (`|FormatText` "체력 : { 0 } \n스피드 : { 1 } \n공격력 : { 2 } \n방어력 : { 3 } \n흡혈량 : { 4 } \n반사량 : { 5 }" (`self.Current_HP`) (`self.SPEED`) (`self.ATK`) (`self.DEF`) (`self.Life_Steal_Amount`) (`self.ReflectiveAmount`))))
  (return))

(fn `UpdateOrbPositions`
  (bind _orbref (`self.OrbRef`))
  ; 구체 배치 최신화하기. 개수에 따라 360에서 나눠서 해당 인덱스 만큼 곱해줘 각도를 구하고 해당 각도를 라디안으로 변환해 반지름 만큼 곱해줘 위치를 지정해줬다.
  (for (_array_element _array_index) _orbref
    (bind _returnvalue (`KismetMathLibrary.Conv_IntToDouble` (* _array_index (/ 360 (`KismetArrayLibrary.Array_Length` _orbref)))))
    (`self.K2_SetActorRelativeRotation` _array_element (`KismetMathLibrary.MakeRotator` 0.0 0.0 _returnvalue) false false)
    (`self.K2_SetActorRelativeLocation` _array_element (`KismetMathLibrary.MakeVector` (* (`KismetMathLibrary.Cos` (`KismetMathLibrary.DegreesToRadians` _returnvalue)) (`self.OrbRadius`)) (* (`KismetMathLibrary.Sin` (`KismetMathLibrary.DegreesToRadians` _returnvalue)) (`self.OrbRadius`))) false false))
  (return))

(fn `UpdateSkill_ID`
  (params (Select :type Integer))
  (locals (BuffSkillData :type "/Game/Data/Structure/SkillData/ST_BuffSkill Structure"))
  (bind (_buffskilldata_increase_amount _buffskilldata_buff_effect) (break `/Game/Data/Structure/SkillData/ST_BuffSkill` (`local.BuffSkillData`)))
  (set `self.Skill_ID` Select)
  (set `local.BuffSkillData` (`|GetArrayItem` (`self.SkillDatas`) (- (`local.Select`) 1)))
  (switch `int` (`local.Select`)
    (:`1`
      (`self.SetHpBuff` (`local.BuffSkillData`)))
    (:`2`
      (`self.SetSpeedBuff` (`local.BuffSkillData`)))
    (:`3`
      (`self.SetAtkBuff` (`local.BuffSkillData`)))
    (:`4`
      (`self.SetAttackLevel`))
    (:`5`
      (`self.MakeOrb`))
    (:`6`
      (`self.SetDefBuff` (`local.BuffSkillData`)))
    (:`7`
      (`self.SetSpeedAndAtkBuff` (`local.BuffSkillData`)))
    (:`8`
      (`self.SetLifeStillAmountBuff` (`local.BuffSkillData`)))
    (:`9`
      (`self.SetReflectiveAmountBuff` (`local.BuffSkillData`)))
    (:`10`
      (`self.SetChainExplosion`)))
  (set `self.PlayerStat` (make `/Game/Data/Structure/PlayerData/ST_PlayerStat` (`self.MaxHP`) (`self.SPEED`) (`self.ATK`) (`self.DEF`) (`self.Life_Steal_Amount`) (`self.Dash Cool Time`) (`self.ReflectiveAmount`)))
  ; 스킬 버프 이펙트
  (`/Engine/EditorBlueprintResources/StandardMacros.IsValid` _buffskilldata_buff_effect
    (:`Is Valid`
      (`NiagaraComponent.SetAsset` (`self.BuffEffect`) _buffskilldata_buff_effect true)
      ; UI 업데이트
      (`self.SendPlayerStat` (`self.PlayerStat`)))
    (:`Is Not Valid`
      (`self.SendPlayerStat` (`self.PlayerStat`)))))

(fn `UserConstructionScript`)
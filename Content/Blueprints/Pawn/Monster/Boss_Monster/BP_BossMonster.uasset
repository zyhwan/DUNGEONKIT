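; Boss monster pawn that loads its stats from the "BossMonster" row of DT_MonsterData and drives an HP bar.
; Attack plays a montage and, on a timer, runs a forward sphere trace that applies ATK damage to the player.
; Incoming damage reduces HP without applying DEF; death disables capsule collision, stops the AI brain, sets the monster state and notifies RoomData.
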(event `self.ReceiveBeginPlay`
  ; 보스 몬스터 스탯 초기화
  (`parent.ReceiveBeginPlay`)
  (set `self.MonsterState` "NewEnumerator4")
  (bind _returnvalue (`|GetDataTableRow` "/Game/Data/DataTable/MonsterData/DT_MonsterData.DT_MonsterData" "BossMonster")
    (:`then`
      (bind _output_get (set `self.MonsterStat` _returnvalue))
      (set `self.MaxHP` (break `/Game/Data/Structure/MonsterData/ST_MonsterStat` _output_get))
      (set `self.HP` (break `/Game/Data/Structure/MonsterData/ST_MonsterStat` _output_get))
      (set `self.ATK` (`.ATK_8_67E03CAC405E344F2042FCBCF524030B` (break `/Game/Data/Structure/MonsterData/ST_MonsterStat` _output_get)))
      (set `CharacterMovementComponent.MaxWalkSpeed` (`.Speed_7_FDD7916F4FF4772C11D320ADE9548B53` (break `/Game/Data/Structure/MonsterData/ST_MonsterStat` _output_get)) (`self.CharacterMovement`))
      (set `self.DEF` (`.Def_10_22A67A904334C017CDC99F9B42B237F6` (break `/Game/Data/Structure/MonsterData/ST_MonsterStat` _output_get)))
      (`/Game/UI/MainGUI/Monster/WBP_MonsterHpBar.SetData` (`self.HP_BAR_Ref`) (`self.HP`) (`self.MaxHP`) 0.0))))

(event `/Game/Interface/BPI_Attack.Attack`
  ; 보스 몬스터 공격 및 데미지 처리
  (set `self.MonsterState` "NewEnumerator5")
  (`|PlayMontage` (`self.Mesh`) "/Game/Blueprints/Pawn/Monster/Boss_Monster/AM_BossMonster.AM_BossMonster" 1.0 0.0 "Attack"
    (:`then`
      (`KismetSystemLibrary.K2_SetTimerDelegate` (delegate `CheckPlayerHit`) 1.0))
    (:`OnCompleted`
      (if (not (`self.IsDead`))
        (set `self.MonsterState` "NewEnumerator6")))))

(event `CheckPlayerHit`
  ; 보스 몬스터 공격 및 데미지 처리
  (bind (_outhits _returnvalue) (`KismetSystemLibrary.SphereTraceMultiForObjects` :`Start` (`self.SetAttackRange` 300.0) :`End` (`self.SetAttackRange` 500.0) :`Radius` 150.0 :`ObjectTypes` (`|MakeArray` "ObjectTypeQuery3" :!type "EObjectTypeQuery Enum") :`DrawDebugType` "ForDuration"))
  (if _returnvalue
    (for _array_element _outhits
      (bind (_bblockinghit _binitialoverlap _time _distance _location _impactpoint _normal _impactnormal _physmat _hitactor) (`GameplayStatics.BreakHitResult` _array_element))
      (if (== (`self.BP PlayerRef`) _hitactor)
        (`GameplayStatics.ApplyDamage` _hitactor (`self.ATK`) null self)
        (break)))))

(event `self.ReceiveAnyDamage`
  (params (Damage :type "Float (single-precision)") (DamageType :type "DamageType Object Reference") (InstigatedBy :type "Controller Object Reference") (DamageCauser :type "Actor Object Reference"))
  (bind _braincomponent (`AIController.BrainComponent` (`AIBlueprintHelperLibrary.GetAIController` self)))
  ; 받은 데미지 처리 및 죽음 처리
  (set `self.HP` (- (`self.HP`) Damage))
  (`/Game/UI/MainGUI/Monster/WBP_MonsterHpBar.SetData` (`self.HP_BAR_Ref`) (`self.HP`) (`self.MaxHP`) Damage)
  (`/Game/UI/MainGUI/Monster/WBP_MonsterHpBar.SetPercent` (`self.HP_BAR_Ref`))
  (if (and (<= (`self.HP`) 0.0) (not (`self.IsDead`)))
    (set `self.IsDead` true)
    (`PrimitiveComponent.SetCollisionEnabled` (`self.CapsuleComponent`) "NoCollision")
    (`/Engine/EditorBlueprintResources/StandardMacros.IsValid` _braincomponent
      (:`Is Valid`
        (`BrainComponent.StopLogic` _braincomponent "Death")
        (set `self.MonsterState` "NewEnumerator2")
        (message `/Game/Interface/BPI_MonsterDead.MonsterDead` (`self.RoomData`))))))

(fn `SetAttackRange`
  (params (RangeValue :type "Float (double-precision)"))
  (returns (Result :type "Vector Structure"))
  (bind (_returnvalue_x _returnvalue_y _returnvalue_z) (`KismetMathLibrary.BreakVector` (+ (`self.K2_GetActorLocation`) (* (`KismetMathLibrary.GetForwardVector` (`self.K2_GetActorRotation`)) (`local.RangeValue`)))))
  (return (`KismetMathLibrary.MakeVector` _returnvalue_x _returnvalue_y (- _returnvalue_z 100.0))))

(fn `UserConstructionScript`
  (`parent.UserConstructionScript`))
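; BP_ADMonster is a monster Blueprint that holds its own combat stats and handles taking damage and dying.
; On BeginPlay it loads MonsterStat from the "ADMonster" row of the DT_MonsterData table.
; AnyDamage subtracts raw damage from HP without applying Def.
; At zero HP or below it sends MonsterDeadMessage through an interface to its owner, the managing room, then destroys itself.
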(event `self.ReceiveBeginPlay`
  ; 초기 스텟 저장
  (`parent.ReceiveBeginPlay`)
  (bind _returnvalue (`|GetDataTableRow` "/Game/Data/DataTable/MonsterData/DT_MonsterData.DT_MonsterData" "ADMonster")
    (:`then`
      (set `self.MonsterStat` _returnvalue))))

(event `self.ReceiveAnyDamage`
  (params (Damage :type "Float (single-precision)") (DamageType :type "DamageType Object Reference") (InstigatedBy :type "Controller Object Reference") (DamageCauser :type "Actor Object Reference"))
  (bind (_monsterstat_hp _monsterstat_atk _monsterstat_speed _monsterstat_def) (break `/Game/Data/Structure/MonsterData/ST_MonsterStat` (`self.MonsterStat`)))
  ; 데미지 로직. 만약 죽을 경우 이 몬스터를 관리하는 방에 인터페이스로 전달
  (bind _output_get (set `self.MonsterStat` (make `/Game/Data/Structure/MonsterData/ST_MonsterStat` (- _monsterstat_hp Damage) _monsterstat_atk _monsterstat_speed _monsterstat_def)))
  (if (<= (break `/Game/Data/Structure/MonsterData/ST_MonsterStat` _output_get) 0.0)
    (message `/Game/Interface/BPI_MonsterDead.MonsterDead` (`self.GetOwner`))
    (`self.K2_DestroyActor`)))

(fn `UserConstructionScript`
  (`parent.UserConstructionScript`))
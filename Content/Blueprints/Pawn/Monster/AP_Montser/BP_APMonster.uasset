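; AP monster pawn: an AI-controlled enemy tied to a room, with data-driven stats and a melee attack on the player.
; BeginPlay loads DT_MonsterData stats, then after a delay passes the room center to the AI Blackboard.
; AnyDamage updates the HP bar; death stops AI logic, notifies the room and plays a montage, adding fire VFX under chain explosion.
; Attack plays a montage, then a timed sphere trace damages only the player.
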(event `self.ReceiveBeginPlay`
  ; AP 몬스터 스탯 캐싱 및 초기 애니메이션 후 블랙보드의 value 값 전달
  (`parent.ReceiveBeginPlay`)
  (`|ExecutionSequence`
    (:`then_0`
      (bind _returnvalue (`|GetDataTableRow` "/Game/Data/DataTable/MonsterData/DT_MonsterData.DT_MonsterData" "APMonster")
        (:`then`
          (bind _output_get (set `self.MonsterStat` _returnvalue))
          (set `self.MaxHP` (break `/Game/Data/Structure/MonsterData/ST_MonsterStat` _output_get))
          (set `self.HP` (break `/Game/Data/Structure/MonsterData/ST_MonsterStat` _output_get))
          (set `self.ATK` (`.ATK_8_67E03CAC405E344F2042FCBCF524030B` (break `/Game/Data/Structure/MonsterData/ST_MonsterStat` _output_get)))
          (set `CharacterMovementComponent.MaxWalkSpeed` (`.Speed_7_FDD7916F4FF4772C11D320ADE9548B53` (break `/Game/Data/Structure/MonsterData/ST_MonsterStat` _output_get)) (`self.CharacterMovement`))
          (set `self.DEF` (`.Def_10_22A67A904334C017CDC99F9B42B237F6` (break `/Game/Data/Structure/MonsterData/ST_MonsterStat` _output_get)))
          (`/Game/UI/MainGUI/Monster/WBP_MonsterHpBar.SetData` (`self.HP_BAR_Ref`) (`self.HP`) (`self.MaxHP`) 0.0))))
    (:`then_1`
      (`KismetSystemLibrary.K2_SetTimer` null "SetBlackBoardCenterLocationValue" 3.0))))

(event `self.ReceiveAnyDamage`
  (params (Damage :type "Float (single-precision)") (DamageType :type "DamageType Object Reference") (InstigatedBy :type "Controller Object Reference") (DamageCauser :type "Actor Object Reference"))
  (bind _braincomponent (`AIController.BrainComponent` (`AIBlueprintHelperLibrary.GetAIController` self)))
  ; 몬스터 입는 데미지 처리 로직
  (set `self.HP` (- (`self.HP`) Damage))
  (`/Game/UI/MainGUI/Monster/WBP_MonsterHpBar.SetData` (`self.HP_BAR_Ref`) (`self.HP`) (`self.MaxHP`) Damage)
  (`/Game/UI/MainGUI/Monster/WBP_MonsterHpBar.SetPercent` (`self.HP_BAR_Ref`))
  (if (<= (`self.HP`) 0.0)
    (set `self.IsDead` true)
    (`self.SetActorEnableCollision` false)
    (`/Engine/EditorBlueprintResources/StandardMacros.IsValid` _braincomponent
      (:`Is Valid`
        (`BrainComponent.StopLogic` _braincomponent "Death")
        (message `/Game/Interface/BPI_MonsterDead.MonsterDead` (`self.RoomData`))
        (if (`/Game/Blueprints/Pawn/Player/BP_Player.IsChainExplosion` (`self.BP PlayerRef`))
          (`NiagaraFunctionLibrary.SpawnSystemAtLocation` "/Game/Assets/Effect/BuffSkill/VFX_Niagara/NS_DeathFireEffect.NS_DeathFireEffect" (`self.K2_GetActorLocation`))
          (`|PlayMontage` (`self.Mesh`) "/Game/Blueprints/Pawn/Monster/AP_Montser/AM_APMonster.AM_APMonster" 1.0 0.0 "Death")
          (else
            (`|PlayMontage` (`self.Mesh`) "/Game/Blueprints/Pawn/Monster/AP_Montser/AM_APMonster.AM_APMonster" 1.0 0.0 "Death")))))))

(event `/Game/Interface/BPI_Attack.Attack`
  ; 공격 로직
  (`|PlayMontage` (`self.Mesh`) "/Game/Blueprints/Pawn/Monster/AP_Montser/AM_APMonster.AM_APMonster" 1.5 0.0 "Attack"
    (:`then`
      (`KismetSystemLibrary.K2_SetTimerDelegate` (delegate `CheckPlayerHit`) 0.8))))

(event `CheckPlayerHit`
  (bind _returnvalue (`self.K2_GetActorLocation`))
  ; 공격 로직
  (bind (_outhits _returnvalue_2) (`KismetSystemLibrary.SphereTraceMultiForObjects` _returnvalue _returnvalue 250.0 (`|MakeArray` "ObjectTypeQuery3" :!type "EObjectTypeQuery Enum")))
  (if _returnvalue_2
    (for _array_element _outhits
      (bind (_bblockinghit _binitialoverlap _time _distance _location _impactpoint _normal _impactnormal _physmat _hitactor) (`GameplayStatics.BreakHitResult` _array_element))
      (if (== (`self.BP PlayerRef`) _hitactor)
        (`GameplayStatics.ApplyDamage` _hitactor (`self.ATK`) null self)
        (break)))))

(fn `SetBlackBoardCenterLocationValue`
  ; AI 블랙보드에 AP방에 중심 좌표 넘겨주기
  (`BlackboardComponent.SetValueAsVector` (`AIBlueprintHelperLibrary.GetBlackboard` (`AIBlueprintHelperLibrary.GetAIController` self)) (`self.Key Name`) (`SceneComponent.K2_GetComponentLocation` (`SceneComponent.GetChildComponent` (`/Game/Blueprints/Dungeon/BP_Dungeon/BP_Master_Room.Center` (`self.RoomData`)) 0))))

(fn `UserConstructionScript`
  (`parent.UserConstructionScript`))
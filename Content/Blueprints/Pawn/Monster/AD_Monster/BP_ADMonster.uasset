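; BP_ADMonster is the AD monster enemy, which loads its stats from DT_MonsterData on BeginPlay and applies the speed to its movement.
; Attack plays a montage, while CheckAttackHit sphere-traces pawns around the monster and damages the referenced player with its ATK, drawing debug shapes.
; Incoming damage subtracts directly from HP, ignoring Def; at zero it notifies its managing room through MonsterDeadMessage and destroys itself.
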(event `self.ReceiveBeginPlay`
  ; 초기 스텟 저장
  (`parent.ReceiveBeginPlay`)
  (bind _returnvalue (`|GetDataTableRow` "/Game/Data/DataTable/MonsterData/DT_MonsterData.DT_MonsterData" "ADMonster")
    (:`then`
      (bind _output_get (set `self.MonsterStat` _returnvalue))
      (set `CharacterMovementComponent.MaxWalkSpeed` (`.Speed_7_FDD7916F4FF4772C11D320ADE9548B53` (break `/Game/Data/Structure/MonsterData/ST_MonsterStat` _output_get)) (`self.CharacterMovement`)))))

(event `self.ReceiveAnyDamage`
  (params (Damage :type "Float (single-precision)") (DamageType :type "DamageType Object Reference") (InstigatedBy :type "Controller Object Reference") (DamageCauser :type "Actor Object Reference"))
  (bind (_monsterstat_hp _monsterstat_atk _monsterstat_speed _monsterstat_def) (break `/Game/Data/Structure/MonsterData/ST_MonsterStat` (`self.MonsterStat`)))
  ; 데미지 로직. 만약 죽을 경우 이 몬스터를 관리하는 방에 인터페이스로 전달
  (bind _output_get (set `self.MonsterStat` (make `/Game/Data/Structure/MonsterData/ST_MonsterStat` (- _monsterstat_hp Damage) _monsterstat_atk _monsterstat_speed _monsterstat_def)))
  (if (<= (break `/Game/Data/Structure/MonsterData/ST_MonsterStat` _output_get) 0.0)
    (message `/Game/Interface/BPI_MonsterDead.MonsterDead` (`self.RoomData`))
    (`self.K2_DestroyActor`)))

(event `CheckAttackHit`
  (bind _returnvalue (`self.K2_GetActorLocation`))
  (bind (_monsterstat_hp _monsterstat_atk) (break `/Game/Data/Structure/MonsterData/ST_MonsterStat` (`self.MonsterStat`)))
  (`KismetSystemLibrary.PrintString` "AD 몬스터 공격!")
  (bind (_outhits _returnvalue_2) (`KismetSystemLibrary.SphereTraceMultiForObjects` :`Start` _returnvalue :`End` _returnvalue :`Radius` 100.0 :`ObjectTypes` (`|MakeArray` "ObjectTypeQuery3" :!type "EObjectTypeQuery Enum") :`DrawDebugType` "ForDuration"))
  (if _returnvalue_2
    (for _array_element _outhits
      (bind (_bblockinghit _binitialoverlap _time _distance _location _impactpoint _normal _impactnormal _physmat _hitactor) (`GameplayStatics.BreakHitResult` _array_element))
      (if (== (`self.BP PlayerRef`) _hitactor)
        (`GameplayStatics.ApplyDamage` _hitactor _monsterstat_atk null self)
        (break)))))

(event `/Game/Interface/BPI_Attack.Attack`
  (`|PlayMontage` (`self.Mesh`) "/Game/Blueprints/Pawn/Monster/AD_Monster/Animations/AM_ADMonster.AM_ADMonster"))

(fn `UserConstructionScript`
  (`parent.UserConstructionScript`))
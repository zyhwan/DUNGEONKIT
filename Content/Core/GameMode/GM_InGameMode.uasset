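; In-game GameMode that procedurally builds a dungeon at BeginPlay and runs room combat flow through to the ending screen.
; Rooms spawn at random open exit arrows, picked by DataTable weight, with line traces rejecting blocked exits.
; A boss room follows, and leftover exits are walled.
; Entering combat rooms triggers delayed wall and monster spawns; clearing removes walls, and the boss room shows the ending UI.
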(event `self.ReceiveBeginPlay`
  ; BeginPlay 초기화
  (`|ExecutionSequence`
    (:`then_0`
      ;; Cached Data
      (`self.SetCachedDungeonData`)
      (`self.SetTotalWeight`)
      (`self.CachedRef`))
    (:`then_1`
      ;; Generate Rooms
      (`self.SpawnStartRoom`)
      (`self.GenerateRooms`)
      (`self.SetBossRoom`)
      (`self.Close Holes`))))

(event `/Game/Interface/BPI_RoomEvent.OnRoomEntered`
  (params (RoomType :type "/Game/Data/Enum/E_RoomType Enum" :default "NewEnumerator1") (ClearCondition :type Boolean) (SendRoomInfo :type "/Game/Blueprints/Dungeon/BP_Dungeon/BP_Master_Room Object Reference"))
  ; 방 감지 로직.
  (switch `/Game/Data/Enum/E_RoomType` RoomType
    (:`NewEnumerator1`
      _)
    (:`NewEnumerator2`
      _)
    (:`NewEnumerator11`
      _))
  (`KismetSystemLibrary.K2_SetTimerDelegate` (delegate `EnterEventTimer`) 1.0))

(event `EnterEventTimer`
  ; 방 감지 로직.
  (`self.SpawnWalls` (stale `/Game/Interface/BPI_RoomEvent.OnRoomEntered` SendRoomInfo) (stale `/Game/Interface/BPI_RoomEvent.OnRoomEntered` ClearCondition))
  (`self.SpawnMonster` (stale `/Game/Interface/BPI_RoomEvent.OnRoomEntered` RoomType) (stale `/Game/Interface/BPI_RoomEvent.OnRoomEntered` SendRoomInfo))
  (`/Game/Blueprints/Pawn/Player/BP_Player.Set_for_a_Moment_Input` (`self.PlayerRef`)))

(event `/Game/Interface/BPI_RoomEvent.OnRoomEndCondition`
  (params (Condition :type Boolean) (RoomType :type "/Game/Data/Enum/E_RoomType Enum" :default "NewEnumerator1"))
  ; 각 방의 클리어 조건 감지 후 클리어된 방의 이벤트
  (`|ExecutionSequence`
    (:`then_0`
      (if Condition
        (for _array_element (`self.TempWalls`)
          (`/Engine/EditorBlueprintResources/StandardMacros.IsValid` _array_element
            (:`Is Valid`
              (`self.K2_DestroyActor` _array_element))))))
    (:`then_1`
      ;; 보스 클리어 시 엔딩 화면
      (if (`|EnumEquality` RoomType "NewEnumerator11")
        (`WidgetBlueprintLibrary.SetInputMode_UIOnlyEx` (`self.PC_Ref`) (`/Game/Core/HUD/BP_GameHUD.EndingGUI` (`/Game/Controller/BP_PlayerController.HUD_Ref` (`self.PC_Ref`))) "LockAlways" true)
        (set `PlayerController.bShowMouseCursor` true (`self.PC_Ref`))
        (`/Game/Core/HUD/BP_GameHUD.ShowEndingGUI` (`/Game/Controller/BP_PlayerController.HUD_Ref` (`self.PC_Ref`)))))))

(fn `CachedRef`
  (bind _asbp_player (cast `/Game/Blueprints/Pawn/Player/BP_Player` (`GameplayStatics.GetPlayerCharacter` 0)))
  (`/Engine/EditorBlueprintResources/StandardMacros.IsValid` _asbp_player
    (:`Is Valid`
      (set `self.PlayerRef` _asbp_player)
      (bind _asbp_player_controller (cast `/Game/Controller/BP_PlayerController` (`GameplayStatics.GetPlayerController` 0)))
      (`/Engine/EditorBlueprintResources/StandardMacros.IsValid` _asbp_player_controller
        (:`Is Valid`
          (set `self.PC_Ref` _asbp_player_controller))))))

(fn `CheckEndLoop`
  (returns (ReturnValue :type Boolean))
  (return (and (> (`self.Room Amount`) 0) (`KismetArrayLibrary.Array_IsNotEmpty` (`self.Exits List`)) (>= (`self.MaxRetry`) (`self.RetryCount`)))))

(fn `CheckOverLapRoom`
  (returns (OverlapCheck :type Boolean))
  (bind _select_exit_point (`self.Select Exit Point`))
  (bind _select_exit_point_2 (`self.Select Exit Point`))
  ; 생성하는 위치
  (set `self.Select Exit Point` (`KismetArrayLibrary.Array_Random` (`self.Exits List`)))
  ; 생성할 곳에 Room이 있는지 체크
  (bind (_outhit _returnvalue) (`KismetSystemLibrary.LineTraceSingle` (+ (`SceneComponent.K2_GetComponentLocation` _select_exit_point_2) (* (`SceneComponent.GetForwardVector` _select_exit_point_2) 50.0)) (+ (`SceneComponent.K2_GetComponentLocation` _select_exit_point) (* (`SceneComponent.GetForwardVector` _select_exit_point) 500.0)) "TraceTypeQuery1"))
  (return _returnvalue))

(fn `Close Holes`
  (for _array_element (`self.Exits List`)
    (`|SpawnActorFromClass` "/Game/Blueprints/Dungeon/BP_Dungeon/BP_End_Wall.BP_End_Wall_C" (`SceneComponent.K2_GetComponentToWorld` _array_element) "AlwaysSpawn" "MultiplyWithRoot" null null))
  (set `self.DungeonComplete` true))

(fn `GenerateDungeonRoom`
  (bind (_selectdungeondata_roomtype _selectdungeondata_roomclass) (break `/Game/Data/Structure/DungeonData/ST_DungeonData` (`self.SelectDungeonData`)))
  ; 가중치를 이용해 AD,AP,Reward,HallWay 생성하기
  (`self.SetDungeonData`)
  ; 뽑은 Room 생성하기
  (bind _returnvalue (`|SpawnActorFromClass` _selectdungeondata_roomclass (`SceneComponent.K2_GetComponentToWorld` (`self.Select Exit Point`)) "AlwaysSpawn" "MultiplyWithRoot" null _selectdungeondata_roomtype null))
  (set `self.Latest Room` _returnvalue)
  (set `self.Room Amount` (- (`self.Room Amount`) 1))
  ;; 한번 생성된 방은 목록에서 삭제한다.
  (`KismetArrayLibrary.Array_RemoveItem` (`self.Exits List`) (`self.Select Exit Point`))
  (`KismetArrayLibrary.Array_Append` (`self.Exits List`) (`SceneComponent.GetChildrenComponents` (`/Game/Blueprints/Dungeon/BP_Dungeon/BP_Master_Room.Exits Folder` (`self.Latest Room`)) false)))

(fn `GenerateRooms`
  (while (`self.CheckEndLoop`) :!label _label
    (bind _overlapcheck (`self.CheckOverLapRoom`))
    (if _overlapcheck
      ; 최대 겹침 횟수 제한, 겹치는 출구 목록에서 제외
      (`/Engine/EditorBlueprintResources/StandardMacros.IncrementInt` (`self.RetryCount`)
        (:`  `
          (`KismetArrayLibrary.Array_RemoveItem` (`self.Exits List`) (`self.Select Exit Point`))
          (goto _label)))
      (else
        (`self.GenerateDungeonRoom`)))))

(fn `SetBossRoom`
  (bind _overlapcheck (`self.CheckOverLapRoom`))
  (if _overlapcheck
    (`KismetArrayLibrary.Array_RemoveItem` (`self.Exits List`) (`self.Select Exit Point`))
    (`self.SetBossRoom`)
    (else
      (`KismetArrayLibrary.Array_RemoveItem` (`self.Exits List`) (`self.Select Exit Point`))
      (bind _returnvalue (`|SpawnActorFromClass` "/Game/Blueprints/Dungeon/BP_Dungeon/BP_Boss_Room.BP_Boss_Room_C" (`SceneComponent.K2_GetComponentToWorld` (`self.Select Exit Point`)) "Undefined" "MultiplyWithRoot" null "NewEnumerator11" null))
      (set `self.Latest Room` _returnvalue)
      (`KismetArrayLibrary.Array_Append` (`self.Exits List`) (`SceneComponent.GetChildrenComponents` (`/Game/Blueprints/Dungeon/BP_Dungeon/BP_Master_Room.Exits Folder` (`self.Latest Room`)) false)))))

(fn `SetCachedDungeonData`
  (bind _outrownames (`DataTableFunctionLibrary.GetDataTableRowNames` "/Game/Data/DataTable/DungeonData/DT_DungeonData.DT_DungeonData"))
  (for _array_element _outrownames
    (bind _returnvalue (`|GetDataTableRow` "/Game/Data/DataTable/DungeonData/DT_DungeonData.DT_DungeonData" _array_element)
      (:`then`
        (`KismetArrayLibrary.Array_Add` (`self.DungeonDataCach`) _returnvalue)))))

(fn `SetDungeonData`
  (set `self.RandomPoint` (`KismetMathLibrary.RandomFloatInRange` 0.0 (`self.TotalWeight`)))
  (for _array_element (`self.DungeonDataCach`)
    (bind _output_get (set `self.SelectDungeonData` _array_element))
    (bind _output_get_2 (set `self.RandomPoint` (- (`self.RandomPoint`) (`.Weight_26_9AD0A3414483E6439D0F2BAF4A882777` (break `/Game/Data/Structure/DungeonData/ST_DungeonData` _output_get)))))
    (if (<= _output_get_2 0.0)
      (break))))

(fn `SetTotalWeight`
  (for _array_element (`self.DungeonDataCach`)
    (set `self.TotalWeight` (+ (`self.TotalWeight`) (`.Weight_26_9AD0A3414483E6439D0F2BAF4A882777` (break `/Game/Data/Structure/DungeonData/ST_DungeonData` _array_element))))))

(fn `SpawnMonster`
  (params (Selection :type "/Game/Data/Enum/E_RoomType Enum" :default "NewEnumerator1") (RoomRef :type "Object Object Reference"))
  (bind _roomref (`local.RoomRef`))
  (switch `/Game/Data/Enum/E_RoomType` Selection
    (:`NewEnumerator1`
      (bind _asbp_dungeon_adroom (cast `/Game/Blueprints/Dungeon/BP_Dungeon/BP_Dungeon_ADRoom` _roomref))
      (`/Engine/EditorBlueprintResources/StandardMacros.IsValid` _asbp_dungeon_adroom
        (:`Is Valid`
          (`/Game/Blueprints/Dungeon/BP_Dungeon/BP_Dungeon_ADRoom.SpawnMonsters` _asbp_dungeon_adroom))))
    (:`NewEnumerator2`
      (bind _asbp_dungeon_aproom (cast `/Game/Blueprints/Dungeon/BP_Dungeon/BP_Dungeon_APRoom` _roomref))
      (`/Engine/EditorBlueprintResources/StandardMacros.IsValid` _asbp_dungeon_aproom
        (:`Is Valid`
          (`/Game/Blueprints/Dungeon/BP_Dungeon/BP_Dungeon_APRoom.SpawnMosnters` _asbp_dungeon_aproom))))
    (:`NewEnumerator11`
      (bind _asbp_boss_room (cast `/Game/Blueprints/Dungeon/BP_Dungeon/BP_Boss_Room` (`local.RoomRef`)))
      (`/Engine/EditorBlueprintResources/StandardMacros.IsValid` _asbp_boss_room
        (:`Is Valid`
          (`/Game/Blueprints/Dungeon/BP_Dungeon/BP_Boss_Room.SpawnBossMonster` _asbp_boss_room))))))

(fn `SpawnStartRoom`
  (bind _returnvalue (`|SpawnActorFromClass` "/Game/Blueprints/Dungeon/BP_Dungeon/BP_Dungeon_StartRoom.BP_Dungeon_StartRoom_C" (`KismetMathLibrary.MakeTransform` (0.0 0.0 0.0) (struct :`Yaw` 45.0)) "Undefined" "MultiplyWithRoot" null "NewEnumerator10" null))
  ; Exits List에 출구 저장
  (`KismetArrayLibrary.Array_Append` (`self.Exits List`) (`SceneComponent.GetChildrenComponents` (`/Game/Blueprints/Dungeon/BP_Dungeon/BP_Master_Room.Exits Folder` _returnvalue) false)))

(fn `SpawnWalls`
  (params (SpawnPoint :type "/Game/Blueprints/Dungeon/BP_Dungeon/BP_Master_Room Object Reference") (Condition :type Boolean) (RoomData :type "/Game/Data/Structure/RoomData/ST_RoomData Structure"))
  (if (not Condition)
    (for _array_element (`SceneComponent.GetChildrenComponents` (`/Game/Blueprints/Dungeon/BP_Dungeon/BP_Master_Room.Exits Folder` SpawnPoint) false)
      (bind _returnvalue (`|SpawnActorFromClass` "/Game/Blueprints/Dungeon/BP_Dungeon/BP_End_Wall.BP_End_Wall_C" (`SceneComponent.K2_GetComponentToWorld` _array_element) "Undefined" "MultiplyWithRoot" null null))
      (`KismetArrayLibrary.Array_Add` (`self.TempWalls`) _returnvalue)
      (for _array_element_2 (`SceneComponent.GetChildrenComponents` (`/Game/Blueprints/Dungeon/BP_Dungeon/BP_Master_Room.Enter Folder` (`local.SpawnPoint`)) false)
        (bind _returnvalue_2 (`|SpawnActorFromClass` "/Game/Blueprints/Dungeon/BP_Dungeon/BP_End_Wall.BP_End_Wall_C" (`SceneComponent.K2_GetComponentToWorld` _array_element_2) "Undefined" "MultiplyWithRoot" null null))
        (`KismetArrayLibrary.Array_Add` (`self.TempWalls`) _returnvalue_2)))))

(fn `UserConstructionScript`)
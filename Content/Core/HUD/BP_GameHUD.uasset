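; Game HUD that creates and owns the player's UI widgets: main stat GUI, skill selection, death fade-out and ending screen.
; On BeginPlay it caches the player controller and character, then binds to the skill-selection and player-stat dispatchers.
; A skill pick updates the player and icon count, then unpauses and closes the selection widget.
; Public functions show death and ending screens and toggle dash alpha.
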(event `self.ReceiveBeginPlay`
  (`self.Cached_Ref`)
  (`|ExecutionSequence`
    (:`then_0`
      ; 디스패처로 받은 어떤 skill을 선택했는지 여부와 이벤트 처리
      (add `/Game/UI/WBP_MainSkillSelectWidget.OnFinalSkillSelected` (`self.SkillUMG`) (delegate `SetSkill_ID_ToPlayer`)))
    (:`then_1`
      ; 플레이어 스탯 정보UI 처리
      (add `/Game/Blueprints/Pawn/Player/BP_Player.SendPlayerStat` (`self.PlayerRef`) (delegate `SendPlayerStatData`)))))

(event `SetSkill_ID_ToPlayer`
  (params (SelectSkill_ID :type Integer))
  ; 디스패처로 받은 어떤 skill을 선택했는지 여부와 이벤트 처리
  (`/Game/Blueprints/Pawn/Player/BP_Player.UpdateSkill_ID` (`self.PlayerRef`) SelectSkill_ID)
  (`/Game/UI/MainGUI/WBP_MainGUI.SetIconCountText` (`self.PlayerStatGUI`) SelectSkill_ID)
  (set `PlayerController.bShowMouseCursor` false (`GameplayStatics.GetPlayerController` 0))
  (`GameplayStatics.SetGamePaused` false)
  (`Widget.RemoveFromParent` (`self.SkillUMG`)))

(event `SendPlayerStatData`
  (params (PlayerStat :type "/Game/Data/Structure/PlayerData/ST_PlayerStat Structure"))
  ; 플레이어 스탯 정보UI 처리
  (`/Game/UI/MainGUI/WBP_MainGUI.SetPlayerStatText` (`self.PlayerStatGUI`) PlayerStat))

(fn `Cached_Ref`
  (bind _asbp_player_controller (cast `/Game/Controller/BP_PlayerController` (`GameplayStatics.GetPlayerController` 0)))
  (`/Engine/EditorBlueprintResources/StandardMacros.IsValid` _asbp_player_controller
    (:`Is Valid`
      (set `self.PC_Ref` _asbp_player_controller)
      (bind _asbp_player (cast `/Game/Blueprints/Pawn/Player/BP_Player` (`GameplayStatics.GetPlayerCharacter` 0)))
      (`/Engine/EditorBlueprintResources/StandardMacros.IsValid` _asbp_player
        (:`Is Valid`
          (set `self.PlayerRef` _asbp_player)
          (bind _returnvalue (`|CreateWidget` "/Game/UI/WBP_MainSkillSelectWidget.WBP_MainSkillSelectWidget_C"))
          (set `self.SkillUMG` _returnvalue)
          (bind _returnvalue_2 (`|CreateWidget` "/Game/UI/MainGUI/WBP_MainGUI.WBP_MainGUI_C"))
          (set `self.PlayerStatGUI` _returnvalue_2)
          (`UserWidget.AddToViewport` _returnvalue_2 0)
          (bind _returnvalue_3 (`|CreateWidget` "/Game/UI/MainGUI/WBP_DeathFadeOut.WBP_DeathFadeOut_C"))
          (set `self.DeathGUI` _returnvalue_3)
          (`UserWidget.AddToViewport` _returnvalue_3 0)
          (`Widget.SetVisibility` (`self.DeathGUI`) "Collapsed")
          (bind _returnvalue_4 (`|CreateWidget` "/Game/UI/MainGUI/WBP_EndingGUI.WBP_EndingGUI_C"))
          (set `self.EndingGUI` _returnvalue_4))))))

(fn `SetDashAlpha0`
  (`/Game/UI/MainGUI/WBP_MainGUI.SetDashAlpha_0` (`self.PlayerStatGUI`)))

(fn `SetDashAlpha1`
  (`/Game/UI/MainGUI/WBP_MainGUI.SetDashAlpha_1` (`self.PlayerStatGUI`)))

(fn `ShowDeathGUI`
  (`WidgetBlueprintLibrary.SetInputMode_UIOnlyEx` (`self.PC_Ref`) (`self.DeathGUI`) "LockAlways" true)
  (set `PlayerController.bShowMouseCursor` true (`self.PC_Ref`))
  (`Widget.SetVisibility` (`self.DeathGUI`) "Visible")
  (`/Game/UI/MainGUI/WBP_DeathFadeOut.FadeOutAnimStart` (`self.DeathGUI`)))

(fn `ShowEndingGUI`
  (`UserWidget.AddToViewport` (`self.EndingGUI`) 0))

(fn `UserConstructionScript`)
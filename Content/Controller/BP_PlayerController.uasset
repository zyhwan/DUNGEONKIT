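; BP_PlayerController is the player controller that sets up Enhanced Input and links room events and player state to the HUD.
; It caches the player and HUD, then forwards health, death screen and uncleared room names to the UI.
; Entering an uncleared reward room or clearing a non-boss room starts a short timer, apparently for DrawSkillSelect.
; DrawSkillSelect shows random skill choices, pauses the game and reveals the cursor.
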(event `self.ReceiveBeginPlay`
  ; 초기 캐싱 작업
  (`WidgetBlueprintLibrary.SetInputMode_GameOnly` self)
  (bind _asbp_player (cast `/Game/Blueprints/Pawn/Player/BP_Player` (`GameplayStatics.GetPlayerPawn` 0)))
  (`/Engine/EditorBlueprintResources/StandardMacros.IsValid` _asbp_player
    (:`Is Valid`
      (set `self.PlayerRef` _asbp_player)
      (`self.SetInputSystem`)
      (bind _asbp_game_hud (cast `/Game/Core/HUD/BP_GameHUD` (`self.GetHUD`)))
      (`/Engine/EditorBlueprintResources/StandardMacros.IsValid` _asbp_game_hud
        (:`Is Valid`
          (set `self.HUD_Ref` _asbp_game_hud))))))

(event `/Game/Interface/BPI_RoomEvent.OnRoomEntered`
  (params (RoomType :type "/Game/Data/Enum/E_RoomType Enum" :default "NewEnumerator1") (ClearCondition :type Boolean) (SendRoomInfo :type "/Game/Blueprints/Dungeon/BP_Dungeon/BP_Master_Room Object Reference"))
  ; 인터페이스로 무슨 타입의 방인지 감지하고 방 이름 출력 및 보상방이면 즉시 스킬 선택
  (switch `/Game/Data/Enum/E_RoomType` RoomType
    (:`NewEnumerator1`
      (if (not ClearCondition)
        (`/Game/UI/MainGUI/WBP_MainGUI.SetRoomName` (`/Game/Core/HUD/BP_GameHUD.PlayerStatGUI` (`self.HUD_Ref`)) RoomType :!label _label)))
    (:`NewEnumerator2`
      (if (not ClearCondition)
        (goto _label)))
    (:`NewEnumerator3`
      (if (not ClearCondition)
        (`self.SetTimer_SkillSelect`)
        (set `/Game/Blueprints/Dungeon/BP_Dungeon/BP_Master_Room.ClearCondition` true SendRoomInfo)
        (goto _label)))))

(event `/Game/Interface/BPI_RoomEvent.OnRoomEndCondition`
  (params (Condition :type Boolean) (RoomType :type "/Game/Data/Enum/E_RoomType Enum" :default "NewEnumerator1"))
  ; 방 클리어 시 보스 방이 아니라면 스킬 선택 이벤트.
  (if (and Condition (`|EnumInequality` RoomType "NewEnumerator11"))
    (`self.SetTimer_SkillSelect`)))

(event `/Game/Interface/BPI_SetPlayerHp.SetPlayerHp`
  (params (CurrentHp :type "Float (double-precision)") (MaxHp :type "Float (double-precision)"))
  ; 플레이어 체력 상태 표시 HUD에서 관리.
  (`/Game/UI/MainGUI/WBP_MainGUI.SetHpBarPercent` (`/Game/Core/HUD/BP_GameHUD.PlayerStatGUI` (`self.HUD_Ref`)) CurrentHp MaxHp))

(fn `DrawSkillSelect`
  (bind _skillumg (`/Game/Core/HUD/BP_GameHUD.SkillUMG` (`self.HUD_Ref`)))
  (`UserWidget.AddToViewport` _skillumg 0)
  (`/Game/UI/WBP_MainSkillSelectWidget.CallSkillSelectImage` _skillumg)
  (`/Game/UI/WBP_MainSkillSelectWidget.SetRandomSkillButton` _skillumg)
  (`GameplayStatics.SetGamePaused` true)
  (set `self.bShowMouseCursor` true))

(fn `SetInputSystem`
  (bind _returnvalue (subsystem `EnhancedInputLocalPlayerSubsystem`))
  (`/Engine/EditorBlueprintResources/StandardMacros.IsValid` _returnvalue
    (:`Is Valid`
      (`EnhancedInputSubsystemInterface.AddMappingContext` _returnvalue "/Game/Inputs/IMC_Player.IMC_Player" 0 (struct)))))

(fn `SetTimer_SkillSelect`
  ; 방에 입장 후 1초 뒤에 스킬 뜨기
  (`KismetSystemLibrary.K2_SetTimerDelegate` (`|CreateDelegate` :!event `DrawSkillSelect`) 1.5))

(fn `StartDeathGUI`
  (`/Game/Core/HUD/BP_GameHUD.ShowDeathGUI` (`self.HUD_Ref`)))

(fn `UserConstructionScript`)